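; BP_HealthPack is a short-lived health pickup that heals the player on touch and expires five seconds after spawning.
; An overlap on HealthCollider casts to BP_Player, adds a fixed amount of Health capped at the maximum, and updates the player's health bar widget directly.
; It then destroys only the HealthPickup component, leaving actor removal to the lifespan timer.
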(event `self.ReceiveBeginPlay`
  (`self.SetLifeSpan` 5.0))

(event `self.HealthCollider.OnComponentBeginOverlap`
  (params (OverlappedComponent :type "PrimitiveComponent Object Reference") (OtherActor :type "Actor Object Reference") (OtherComp :type "PrimitiveComponent Object Reference") (OtherBodyIndex :type Integer) (bFromSweep :type Boolean) (SweepResult :type "HitResult Structure (by ref)"))
  ;[1 1 1] HealthPack Collision and Update
  (bind _asbp_player (cast `/Game/InfiniteMatrix/Blueprints/BP_Player` OtherActor))
  (bind _output_get (set `/Game/InfiniteMatrix/Blueprints/BP_Player.Health` (`KismetMathLibrary.FMin` (+ (`/Game/InfiniteMatrix/Blueprints/BP_Player.Health` _asbp_player) 10.0) 100.0) _asbp_player))
  (`/Game/InfiniteMatrix/UI/WBP_HealthBar.UpdateHealthBar` (`/Game/InfiniteMatrix/Blueprints/BP_Player.WBPHealthBar` _asbp_player) _output_get)
  (`ActorComponent.K2_DestroyComponent` (`self.HealthPickup`)))

(fn `UserConstructionScript`)