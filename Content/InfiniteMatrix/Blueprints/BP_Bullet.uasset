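; BP_Bullet is a projectile actor that travels along world X at a speed tied to the player's progress.
; Each tick it looks up BP_Player and offsets itself by a frame-rate-independent step built from the player's forward speed, a score-scaled bonus and a fixed extra speed.
; It destroys itself on any actor overlap, or expires through a short lifespan set on BeginPlay.
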(event `self.ReceiveBeginPlay`
  (`self.SetLifeSpan` 5.0))

(event `self.ReceiveActorBeginOverlap`
  (params (OtherActor :type "Actor Object Reference"))
  (`self.K2_DestroyActor`))

(event `self.ReceiveTick`
  (params (DeltaSeconds :type "Float (single-precision)"))
  (bind _returnvalue (`GameplayStatics.GetActorOfClass` "/Game/InfiniteMatrix/Blueprints/BP_Player.BP_Player_C"))
  (`self.K2_AddActorWorldOffset` (`KismetMathLibrary.MakeVector` (* DeltaSeconds (+ (+ (`/Game/InfiniteMatrix/Blueprints/BP_Player.FowardSpeed` _returnvalue) (* (`/Game/InfiniteMatrix/Blueprints/BP_Player.Score` _returnvalue) 25)) 1000.0)))))

(fn `UserConstructionScript`)